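; Automated turret that tracks characters seen by PawnSensing and fires at them while it has ammo, showing ammo and health on a widget screen.
; Tick interpolates tray yaw and cylinder pitch toward the target; a retriggerable delay clears detection when sightings stop.
; A gate with a delayed re-entry loop drives firing: ammo decrement, muzzle flash, sound, bullet trail and socket spawns.
; Hits use a forward line trace, damaging FirstPersonCharacter but only printing for BP_bot.
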(event OnSeePawn(PawnSensing)
  (params (Pawn :type Pawn%20Object%20Reference))
  ;[1 1 1] check enemy area
  (bind _ascharacter (Utilities|Casting|CastToCharacter Pawn))
  (Variables|Default|Setplayer _ascharacter)
  (Utilities|FlowControl|Sequence
    (:then_0
      (Variables|Default|Setin%20range true))
    (:then_1
      (Utilities|FlowControl|RetriggerableDelay 0.15)
      (Variables|Default|Setin%20range false))))

(event Custom|Turret%20rotation
  (bind _player (Variables|Default|Getplayer))
  (bind _turret_tray (Variables|Default|Getturret_tray))
  (bind _delta_time (Variables|Default|Getdelta%20time))
  (bind _player_2 (Variables|Default|Getplayer))
  (bind _turret_tray_2 (Variables|Default|Getturret_tray))
  (bind _rotation_speed (Variables|Default|Getrotation%20speed))
  (bind _returnvalue (Transformation|GetActorLocation _player_2))
  (bind _returnvalue_2 (Transformation|GetWorldLocation _turret_tray))
  (bind _returnvalue_3 (Transformation|GetActorLocation _player))
  (bind _returnvalue_4 (Transformation|GetWorldRotation _turret_tray_2))
  (bind _returnvalue_5 (Math|Rotator|FindLookatRotation _returnvalue_2 _returnvalue_3))
  (bind _yaw (Math|Rotator|BreakRotator _returnvalue_5))
  (bind _returnvalue_6 (Math|Interpolation|RInterpTo (Math|Rotator|MakeRotator 0.0 0.0 (.yaw _returnvalue_4)) (Math|Rotator|MakeRotator 0.0 0.0 _yaw) _delta_time _rotation_speed))
  (if (Variables|Default|Getin%20range)
    (Utilities|FlowControl|Sequence
      (:then_0
        ;[1 0.6073 0.2872] Z rotation turret
        (if (not (Math|Vector|Equal(Vector) _returnvalue_3 "0, 0, 0" 0.0001))
          (CallFunction|SetZworlLocationMulti (Variables|Default|Getturret_tray) (.roll (Variables|Default|GetGet%20Base%20Position)) (.yaw _returnvalue_6))))
      (:then_1
        ;[1 0.8868 0.237] Y rotation turret
        (if (not (Math|Vector|Equal(Vector) _returnvalue "0, 0, 0" 0.0001))
          (CallFunction|SetYWorldLocationMulti (Variables|Default|Getturret_cylinder) (+ (.yaw _returnvalue_6) 1.8e+02) (.pitch (Math|Interpolation|RInterpTo (Transformation|GetWorldRotation (Variables|Default|Getturret_cylinder)) (Math|Rotator|MakeRotator 0.0 (* (.Pitch (Math|Rotator|BreakRotator (Math|Rotator|FindLookatRotation (Transformation|GetWorldLocation (Variables|Default|Getturret_cylinder)) _returnvalue))) -1.0) 0.0) (Variables|Default|Getdelta%20time) (Variables|Default|Getrotation%20speed)))))))))

(event Custom|fire%20action
  ;[1 1 1] fire action
  (if (Variables|Default|Getin%20range)
    (if (== (Variables|Default|Getammo) 0)
      (Utilities|FlowControl|Sequence
        (:then_0
          (goto _label Close))
        (:then_1
          ;;[0.1586 1 0.1772] Custom Turret
          (|soundeffect) ; enters at no ammo pin
        ))
      (else
        (|barrel_rotation)
        (Utilities|FlowControl|Sequence
          (:then_0
            (Utilities|FlowControl|Gate true :!label _label
              (:Exit
                (Utilities|FlowControl|Sequence
                  (:then_0
                    (Utilities|FlowControl|RetriggerableDelay 0.2)
                    (goto _label))
                  (:then_1
                    (|decrementeammo_2)
                    (CallFunction|FireMulti (Variables|Default|Getammo)))))))
          (:then_1
            (goto _label Open)))))
    (else
      (goto _label Close))))

(event Custom|setZworlLocation%20multi
  (params (Target :type Scene%20Component%20Object%20Reference) (New%20Rotation%20X%20%28Roll%29 :type Float%20%28single-precision%29) (New%20Rotation%20Z%20%28Yaw%29 :type Float%20%28single-precision%29))
  ;[1 0.6073 0.2872] Z rotation turret
  (Transformation|SetWorldRotation (Variables|Default|Getturret_tray) (Math|Rotator|MakeRotator New%20Rotation%20X%20%28Roll%29 0.0 New%20Rotation%20Z%20%28Yaw%29) false false))

(event Custom|setYWorldLocation%20multi
  (params (Target :type Scene%20Component%20Object%20Reference) (New%20Rotation%20Z%20%28Yaw%29 :type Float%20%28single-precision%29) (New%20Rotation%20Y%20%28Pitch%29 :type Float%20%28single-precision%29))
  ;[1 0.8868 0.237] Y rotation turret
  (Transformation|SetWorldRotation (Variables|Default|Getturret_cylinder) (Math|Rotator|MakeRotator 0.0 New%20Rotation%20Y%20%28Pitch%29 New%20Rotation%20Z%20%28Yaw%29) false false))

(event Custom|fire%20multi
  (params (ammo :type Integer))
  ;[1 1 1] fire action
  (Variables|Default|Setammo ammo)
  (Utilities|FlowControl|Sequence
    (:then_0
      ;;[0.1586 1 0.1772] Custom Turret
      (|particuleeffect_2))
    (:then_1
      (|soundeffect))
    (:then_2
      (|Aim/Target))
    (:then_3
      (|bullet_trace)
      (|Spawn_Socket))))

(event EventTick
  (params (DeltaSeconds :type Float%20%28single-precision%29))
  (Variables|Default|Setdelta%20time DeltaSeconds)
  (if (not (Variables|Default|GetOFF))
    (CallFunction|TurretRotation)
    (CallFunction|FireAction)
    (Variables|/Game/automatic_turret/UI/turret_screen.Turret_Screen_C|Setammo%20 (stale EventBeginPlay _returnvalue) (Variables|Default|Getammo))
    (Variables|/Game/automatic_turret/UI/turret_screen.Turret_Screen_C|SetMax%20Ammo (stale EventBeginPlay _returnvalue) (Variables|Default|Getmax%20ammo))
    (Variables|/Game/automatic_turret/UI/turret_screen.Turret_Screen_C|Sethealth (stale EventBeginPlay _returnvalue) (Variables|Default|GetHealth))))

(event EventBeginPlay
  (bind _returnvalue (UserInterface|CreateWidget "/Game/automatic_turret/UI/turret_screen.Turret_Screen_C"))
  (UserInterface|SetWidget (Variables|Default|GetWidget) _returnvalue)
  (Variables|Default|SetGet%20Base%20Position (Transformation|GetWorldRotation (Variables|Default|GetDefaultSceneRoot))))

(fn ConstructionScript)

(fn ForwardinTrace
  (bind _arrow (Variables|Default|GetArrow))
  (bind _returnvalue (Transformation|GetWorldLocation _arrow))
  (bind (_outhit _returnvalue_2) (Collision|LineTraceByChannel _returnvalue (+ _returnvalue (* (Math|Vector|GetForwardVector _arrow) (Variables|/Script/AIModule.PawnSensingComponent|GetSightRadius (Variables|Default|GetPawnSensing)))) "TraceTypeQuery2" false 0 "None"))
  (return _outhit _returnvalue_2))