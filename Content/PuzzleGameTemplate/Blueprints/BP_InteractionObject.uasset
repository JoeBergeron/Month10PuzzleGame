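; BP_InteractionObject is a physics object that can be rewound in time when the player's FirstPersonCharacter activates time reverse.
; Each tick it adds Direction to the mesh's linear velocity, then records the mesh transform and velocities into two arrays while time runs normally.
; During reversal it applies and pops the last entries, keeping the oldest one.
; Linear and angular velocity share one Transform array, stored in its Location and Scale fields.
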(event EventBeginPlay
  ;[1 1 1] EventBeginPlay
  (bind _asfirst_person_character (Utilities|Casting|CastToFirstPersonCharacter (Game|GetPlayerCharacter 0)))
  (Variables|Default|SetCharacter _asfirst_person_character))

(event EventTick
  (params (DeltaSeconds :type Float%20%28single-precision%29))
  (bind _character (Variables|Default|GetCharacter))
  (bind _staticmech (Variables|Default|GetStaticMech))
  (bind _velocityarray (Variables|Default|GetVelocityArray))
  (bind _transformarray (Variables|Default|GetTransformArray))
  (bind _velocityarray_2 (Variables|Default|GetVelocityArray))
  (bind _returnvalue (Utilities|Array|LastIndex _transformarray))
  (bind _returnvalue_2 (Utilities|Array|LastIndex _velocityarray_2))
  (bind _timereverseactive (Variables|/Game/PuzzleGameTemplate/Blueprints/FirstPersonCharacter.FirstPersonCharacter_C|GetTimeReverseActive _character))
  (bind _output (Utilities|Array|Get(acopy) _velocityarray _returnvalue_2))
  (bind (_location _rotation _scale) (Math|Transform|BreakTransform _output))
  (Utilities|FlowControl|Sequence
    (:then_0
      ;[1 1 1] Get and Set StaticMesh Physics Linear Velocity
      (bind _returnvalue_3 (Physics|GetPhysicsLinearVelocity (Variables|Default|GetStaticMech) "None"))
      (Physics|SetPhysicsLinearVelocity (Variables|Default|GetStaticMech) (+ _returnvalue_3 (Variables|Default|GetDirection)) false "None"))
    (:then_1
      ;[1 1 1] Set World Transftom\Time reverse event
      (Utilities|FlowControl|Sequence
        (:then_0
          (if _timereverseactive
            (Transformation|SetWorldTransform (Variables|Default|GetStaticMech) (Utilities|Array|Get(acopy) (Variables|Default|GetTransformArray) _returnvalue) false false)
            (if (> _returnvalue 0)
              (Utilities|Array|RemoveIndex (Variables|Default|GetTransformArray) _returnvalue))
            (else
              (Utilities|Array|Add (Variables|Default|GetTransformArray) (Transformation|GetWorldTransform (Variables|Default|GetStaticMech))))))
        (:then_1
          ;[1 1 1] TimeReverseEvent
          (if _timereverseactive
            (Physics|SetPhysicsLinearVelocity (Variables|Default|GetStaticMech) _location false "None")
            (Class|PrimitiveComponent|SetPhysicsAngularVelocityinDegrees (Variables|Default|GetStaticMech) _scale false "None")
            (if (> _returnvalue_2 0)
              (Utilities|Array|RemoveIndex (Variables|Default|GetVelocityArray) _returnvalue_2))
            (else
              (bind _returnvalue_4 (Physics|GetPhysicsLinearVelocity _staticmech "None"))
              (Utilities|Array|Add (Variables|Default|GetVelocityArray) (Math|Transform|MakeTransform _returnvalue_4 "0, 0, 0" (Physics|GetPhysicsAngularVelocityinDegrees _staticmech "None"))))))))))

(fn ConstructionScript)