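; BP_Portal2 is a portal actor that teleports the first-person character to the BP_Portal on overlap.
; When a FirstPersonCharacter enters its box, it finds every BP_Portal and moves the player pawn to that portal's arrow location and facing, playing a passage sound.
; Because it loops over all BP_Portal instances, the last one found is the final destination if several exist.
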(event OnComponentBeginOverlap(Box)
  (params (OverlappedComponent :type Primitive%20Component%20Object%20Reference) (OtherActor :type Actor%20Object%20Reference) (OtherComp :type Primitive%20Component%20Object%20Reference) (OtherBodyIndex :type Integer) (bFromSweep :type Boolean) (SweepResult :type Hit%20Result%20Structure%20%28by%20ref%29))
  ;[1 1 1] When Character overlap portal collision, he teleported to another  portal
  (Utilities|Casting|CastToFirstPersonCharacter OtherActor)
  (bind _outactors (Actor|GetAllActorsOfClass "/Game/PuzzleGameTemplate/Blueprints/BP_Portal.BP_Portal_C"))
  (for _array_element _outactors
    (Transformation|Teleport (Pawn|GetControlledPawn (Game|GetPlayerController 0)) (Transformation|GetWorldLocation (Variables|/Game/PuzzleGameTemplate/Blueprints/BP_Portal.BP_Portal_C|GetArrow _array_element)) (Math|Conversions|RotationFromXVector (Math|Vector|GetForwardVector (Variables|/Game/PuzzleGameTemplate/Blueprints/BP_Portal.BP_Portal_C|GetArrow _array_element))))
    (Audio|Components|Audio|Play (Variables|Default|GetPassage_Through_The_Portal) 0.0)))

(fn ConstructionScript)