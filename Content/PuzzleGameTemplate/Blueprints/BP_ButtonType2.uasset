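; Pressure-plate style puzzle button that is pushed while a Player or InteractionObject tagged actor overlaps its Box.
; Begin overlap plays the ButtonMovement timeline, offsetting the cube mesh from ButtonLocation and setting Pushed true.
; End overlap reverses a separate timeline, Timeline_0, which drives the mesh location and sets Pushed false.
; Overlapping actors are not counted, so any qualifying actor leaving triggers the release.
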(event OnComponentBeginOverlap(Box)
  (params (OverlappedComponent :type Primitive%20Component%20Object%20Reference) (OtherActor :type Actor%20Object%20Reference) (OtherComp :type Primitive%20Component%20Object%20Reference) (OtherBodyIndex :type Integer) (bFromSweep :type Boolean) (SweepResult :type Hit%20Result%20Structure%20%28by%20ref%29))
  ;[1 1 1] The button responds to an Interactive object that has a "InteractionObject" or "Player" tag. When a button interacts with an Interactive Object, the “Pushed” variable becomes true.
  (if (Actor|ActorHasTag OtherActor "InteractionObject")
    (bind _newtrack_0 (Timeline|ButtonMovement Play)
      (:Update
        (Transformation|SetRelativeLocation (Variables|Default|Get1M_Cube_Chamfer) (+ _newtrack_0 (Variables|Default|GetButtonLocation)) false false)
        (Variables|Default|SetPushed true)))
    (elif (Actor|ActorHasTag OtherActor "Player")
      (Timeline|ButtonMovement Play))))

(event OnComponentEndOverlap(Box)
  (params (OverlappedComponent :type Primitive%20Component%20Object%20Reference) (OtherActor :type Actor%20Object%20Reference) (OtherComp :type Primitive%20Component%20Object%20Reference) (OtherBodyIndex :type Integer))
  ;[1 1 1] If the Interactive Object or Player is removed from the Button, the "Pushed" variable becomes false again.
  (if (Actor|ActorHasTag OtherActor "InteractionObject")
    (bind _newtrack_0 (Timeline|Timeline_0 Reverse)
      (:Update
        (Transformation|SetRelativeLocation (Variables|Default|Get1M_Cube_Chamfer) (+ _newtrack_0 (Variables|Default|GetButtonLocation)) false false)
        (Variables|Default|SetPushed false)))
    (elif (Actor|ActorHasTag OtherActor "Player")
      (Timeline|Timeline_0 Reverse))))

(fn ConstructionScript)