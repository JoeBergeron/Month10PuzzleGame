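; BP_InteractionObjectSpawner is a puzzle spawner actor that produces BP_InteractionObject actors while a button is pushed.
; A Delay on Tick makes it check roughly every two seconds, polling the first BP_Button and first BP_ButtonType2 found via GetAllActorsOfClass at a hardcoded index.
; Each pushed button spawns its own object at the SMWindowFrame component's location, ignoring collisions.
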(event EventTick
  (params (DeltaSeconds :type Float%20%28single-precision%29))
  ;[1 1 1] InteractionObjectSpawner spawn Interaction Object, when it determines that a variable is "pushed" in a BP_Button, it becomes true. And it ceases to spawn objects when the variable becomes false again.
  (Utilities|FlowControl|Delay 2.0)
  (Utilities|FlowControl|Sequence
    (:then_0
      (bind _outactors (Actor|GetAllActorsOfClass "/Game/PuzzleGameTemplate/Blueprints/BP_Button.BP_Button_C"))
      (bind _asbp_button (Utilities|Casting|CastToBP_Button (Utilities|Array|Get(acopy) _outactors)))
      (if (Variables|/Game/PuzzleGameTemplate/Blueprints/BP_Button.BP_Button_C|GetPushed _asbp_button)
        (Game|SpawnActorfromClass "/Game/PuzzleGameTemplate/Blueprints/BP_InteractionObject.BP_InteractionObject_C" (Math|Conversions|ToTransform(Vector) (Transformation|GetWorldLocation (Variables|Default|GetSM_WindowFrame))) "AlwaysSpawn" 0 0)))
    (:then_1
      (bind _outactors_2 (Actor|GetAllActorsOfClass "/Game/PuzzleGameTemplate/Blueprints/BP_ButtonType2.BP_ButtonType2_C"))
      (bind _asbp_button_type_2 (Utilities|Casting|CastToBP_ButtonType2 (Utilities|Array|Get(acopy) _outactors_2)))
      (if (Variables|/Game/PuzzleGameTemplate/Blueprints/BP_ButtonType2.BP_ButtonType2_C|GetPushed _asbp_button_type_2)
        (Game|SpawnActorfromClass "/Game/PuzzleGameTemplate/Blueprints/BP_InteractionObject.BP_InteractionObject_C" (Math|Conversions|ToTransform(Vector) (Transformation|GetWorldLocation (Variables|Default|GetSM_WindowFrame))) "AlwaysSpawn" 0 0)))))

(fn ConstructionScript)