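; BP_TimeStopPortal is a trigger volume that nearly freezes world time while the first-person character is inside it.
; Entering the Box drops global time dilation to near zero, then, after a tiny delay, raises the player pawn's custom dilation inversely so it keeps normal speed.
; Leaving restores both dilations after the same delay.
; An entry sound plays, along with a portal cue that stops on exit.
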(event OnComponentBeginOverlap(Box)
  (params (OverlappedComponent :type Primitive%20Component%20Object%20Reference) (OtherActor :type Actor%20Object%20Reference) (OtherComp :type Primitive%20Component%20Object%20Reference) (OtherBodyIndex :type Integer) (bFromSweep :type Boolean) (SweepResult :type Hit%20Result%20Structure%20%28by%20ref%29))
  ;[1 1 1] Set Time Stop
  (Utilities|Casting|CastToFirstPersonCharacter OtherActor)
  (Audio|Components|Audio|Play (Variables|Default|GetTimePortalSound) 0.0)
  (Utilities|Time|SetGlobalTimeDilation 0.0001)
  (Utilities|FlowControl|Delay 0.0001)
  (Variables|/Script/Engine.Actor|SetCustomTimeDilation (Game|Player|GetPlayerPawn 0) 1e+04)
  (Audio|Components|Audio|Play (Variables|Default|Getstopportal_Cue) 0.0))

(event OnComponentEndOverlap(Box)
  (params (OverlappedComponent :type Primitive%20Component%20Object%20Reference) (OtherActor :type Actor%20Object%20Reference) (OtherComp :type Primitive%20Component%20Object%20Reference) (OtherBodyIndex :type Integer))
  ;[1 1 1] Return To Normal Time
  (Utilities|Casting|CastToFirstPersonCharacter OtherActor)
  (Utilities|FlowControl|Delay 0.0001)
  (Utilities|Time|SetGlobalTimeDilation 1.0)
  (Variables|/Script/Engine.Actor|SetCustomTimeDilation (Game|Player|GetPlayerPawn 0) 1.0)
  (Audio|Components|Audio|Stop (Variables|Default|Getstopportal_Cue)))

(fn ConstructionScript)