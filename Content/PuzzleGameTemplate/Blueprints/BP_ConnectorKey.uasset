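; BP_ConnectorKey is a puzzle key actor that detects whether it has clear line of sight to an interaction connector.
; On BeginPlay it loops over all BP_InteractionObjectConnector actors and keeps the last one found.
; Each Tick it line-traces on Visibility, with debug drawing, from its Arrow to that connector's mesh.
; The hit result sets the Connect flag and swaps the Wall400x400 material between connected and red versions.
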(event EventBeginPlay
  ;[1 1 1] EventBeginPlay
  (bind _outactors (Actor|GetAllActorsOfClass "/Game/PuzzleGameTemplate/Blueprints/BP_InteractionObjectConnector.BP_InteractionObjectConnector_C"))
  (for _array_element _outactors
    (Variables|Default|SetInteractionConnector _array_element)))

(event EventTick
  (params (DeltaSeconds :type Float%20%28single-precision%29))
  (bind _wall_400x400 (Variables|Default|GetWall_400x400))
  ;[1 1 1] ConnectToInteractionConnector
  (bind _outhit (Collision|LineTraceByChannel (Transformation|GetWorldLocation (Variables|Default|GetArrow)) (Transformation|GetWorldLocation (Variables|/Game/PuzzleGameTemplate/Blueprints/BP_InteractionObjectConnector.BP_InteractionObjectConnector_C|GetStaticMech (Variables|Default|GetInteractionConnector))) "TraceTypeQuery1" true 0 "ForOneFrame"))
  (if (== (.HitActor (Collision|BreakHitResult _outhit)) (Variables|Default|GetInteractionConnector))
    (Variables|Default|SetConnect true)
    (Rendering|Material|SetMaterial _wall_400x400 0 "/Game/PuzzleGameTemplate/StarterContent/Materials/M_ConnectorKeyMat.M_ConnectorKeyMat")
    (else
      (Variables|Default|SetConnect false)
      (Rendering|Material|SetMaterial _wall_400x400 0 "/Game/PuzzleGameTemplate/StarterContent/Materials/M_ConnectorKeyMatRed.M_ConnectorKeyMatRed"))))

(fn ConstructionScript)